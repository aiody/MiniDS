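; BP_Weber is the player-controlled Weber character, drawn with a flipbook sprite.
; Axis inputs drive forward and right movement plus controller yaw, and cache the movement values in AxisX and AxisY.
; Each tick, UpdateAnimation picks the idle, side, up or down flipbook from those values, with vertical input overriding side.
; Sideways input yaws the sprite to either side, so one side-run flipbook serves both directions.
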(event `self.ReceiveTick`
  (params (DeltaSeconds :type "Float (single-precision)"))
  (`self.UpdateAnimation`))

(event `InputAxis|UpDown`
  (params (AxisValue :type "Float (single-precision)"))
  (`self.AddMovementInput` (`self.GetActorForwardVector`) AxisValue)
  (set `self.AxisY` AxisValue))

(event `InputAxis|LeftRight`
  (params (AxisValue :type "Float (single-precision)"))
  (`self.AddMovementInput` (`self.GetActorRightVector`) AxisValue)
  (set `self.AxisX` AxisValue))

(event `InputAxis|Yaw`
  (params (AxisValue :type "Float (single-precision)"))
  (`self.AddControllerYawInput` AxisValue))

(event `UpdateAnimation`
  (if (and (== (`self.AxisX`) 0.0) (== (`self.AxisY`) 0.0))
    (`PaperFlipbookComponent.SetFlipbook` (`self.Sprite`) "/Game/Animation/Weber/idle/WeberIdle.WeberIdle")
    (else
      (`/Engine/EditorBlueprintResources/StandardMacros.CompareFloat` (`self.AxisX`)
        (:`>`
          (`SceneComponent.K2_SetRelativeRotation` (`self.Sprite`) (`KismetMathLibrary.MakeRotator` 0.0 0.0 90.0) false false)
          (`PaperFlipbookComponent.SetFlipbook` (`self.Sprite`) "/Game/Animation/Weber/run_side/WeberRunSide.WeberRunSide" :!label _label))
        (:`==`
          _)
        (:`<`
          (`SceneComponent.K2_SetRelativeRotation` (`self.Sprite`) (`KismetMathLibrary.MakeRotator` 0.0 0.0 -90.0) false false)
          (goto _label)))
      (`/Engine/EditorBlueprintResources/StandardMacros.CompareFloat` (`self.AxisY`)
        (:`>`
          (`PaperFlipbookComponent.SetFlipbook` (`self.Sprite`) "/Game/Animation/Weber/run_up/WeberRunUp.WeberRunUp"))
        (:`<`
          (`PaperFlipbookComponent.SetFlipbook` (`self.Sprite`) "/Game/Animation/Weber/run_down/WeberRunDown.WeberRunDown"))))))

(fn `UserConstructionScript`)